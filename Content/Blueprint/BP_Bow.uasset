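; BP_Bow is an arrow projectile actor that damages BP_CombatEnemy actors it overlaps.
; LauckArrow attaches a Niagara effect, adds a gravity-free ProjectileMovement component at runtime with scaled velocity, and enables capsule collision.
; It then immediately attempts to attach to the hit actor from the capsule overlap's sweep result, though that overlap event runs no logic.
; Actor overlap applies damage and prints a debug message.
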(event OnComponentBeginOverlap(Capsule)
  (params (OverlappedComponent :type Primitive%20Component%20Object%20Reference) (OtherActor :type Actor%20Object%20Reference) (OtherComp :type Primitive%20Component%20Object%20Reference) (OtherBodyIndex :type Integer) (bFromSweep :type Boolean) (SweepResult :type Hit%20Result%20Structure%20%28by%20ref%29)))

(event Custom|LauckArrow
  (params (Velocity :type Vector))
  (Niagara|SpawnSystemAttached "/Game/Variant_Combat/VFX/NS_Arrow.NS_Arrow" (Variables|Default|GetArrow) "None" "0, 0, 0" "0, 0, 0" "KeepRelativeOffset" false)
  (bind _returnvalue (AddComponent|AddProjectileMovementComponent))
  (bind _output_get (Variables|Default|SetProjectileMovement%20f _returnvalue))
  (Variables|/Script/Engine.MovementComponent|SetVelocity _output_get (* Velocity 3e+03))
  (Variables|/Script/Engine.ProjectileMovementComponent|SetProjectileGravityScale _returnvalue 0.0)
  (Collision|SetCollisionEnabled (Variables|Default|GetCapsule) "QueryAndPhysics")
  (Transformation|AttachActorToActor (.HitActor (Collision|BreakHitResult (stale OnComponentBeginOverlap(Capsule) SweepResult))) "None" "KeepWorld" "KeepWorld" "KeepWorld" true)
  (Actor|SetLifeSpan 0.0))

(event Collision|EventActorBeginOverlap
  (params (OtherActor :type Actor%20Object%20Reference))
  (Utilities|FlowControl|Sequence
    (:then_0
      (bind _asbp_combat_enemy (Utilities|Casting|CastToBP_CombatEnemy OtherActor))
      (bind _returnvalue (Game|Damage|ApplyDamage _asbp_combat_enemy 1.0 (Game|GetPlayerController 0) self "/Script/Engine.DamageType"))
      (Development|PrintString "enneims touché " true true "(R=0.000000,G=0.660000,B=1.000000,A=1.000000)" _returnvalue))))

(event EventTick
  (params (DeltaSeconds :type Float%20%28single-precision%29)))

(event EventBeginPlay)

(fn ConstructionScript)
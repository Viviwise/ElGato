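; BP_ExplosifBaril is an explosive barrel that detonates when a BP_Bow actor hits it.
; On that hit it spawns a scaled-up particle effect and sound at the impact point, fires its RadialForce impulse and applies full radial damage around itself.
; After a short delay it deactivates the emitter and destroys itself.
; BeginPlay also caches its owner as a Character, which the explosion logic never uses.
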(event Collision|EventActorBeginOverlap
  (params (OtherActor :type Actor%20Object%20Reference)))

(event EventTick
  (params (DeltaSeconds :type Float%20%28single-precision%29)))

(event Collision|EventHit
  (params (MyComp :type Primitive%20Component%20Object%20Reference) (Other :type Actor%20Object%20Reference) (OtherComp :type Primitive%20Component%20Object%20Reference) (bSelfMoved :type Boolean) (HitLocation :type Vector :default "0, 0, 0") (HitNormal :type Vector :default "0, 0, 0") (NormalImpulse :type Vector :default "0, 0, 0") (Hit :type Hit%20Result%20Structure%20%28by%20ref%29))
  (Utilities|Casting|CastToBP_Bow Other)
  (bind _returnvalue (Effects|SpawnEmitteratLocation "/Engine/Tutorial/SubEditors/TutorialAssets/TutorialParticleSystem.TutorialParticleSystem" HitLocation "0, 0, 0" "3.000000,3.000000,3.000000"))
  (Audio|PlaySoundatLocation "/Engine/EditorSounds/GamePreview/PossessPlayer.PossessPlayer" HitLocation "0, 0, 0" 1.0 1.0 0.0 0 0 0 0)
  (Class|RadialForceComponent|FireImpulse (Variables|Default|GetRadialForce))
  (Game|Damage|ApplyRadialDamage 5e+01 (Transformation|GetActorLocation self) 5e+02 "/Script/Engine.DamageType" 0 0 0 true "ECC_Visibility")
  (Utilities|FlowControl|Delay 0.5)
  (Components|Activation|Deactivate _returnvalue)
  (Actor|DestroyActor))

(event EventBeginPlay
  (bind _ascharacter (Utilities|Casting|CastToCharacter (Components|GetOwner)))
  (Variables|Default|SetAs%20Character _ascharacter))

(fn ConstructionScript)
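; Player sword attack ability that cycles through combo montages on the combat input.
; On BeginPlay, after a short delay, it spawns a BP_Sword, attaches it hidden to the character mesh's sword socket.
; While active and not mid-attack, input reveals the sword and plays the next montage; otherwise input hides it.
; StartAbility and StopAbility only add logging; an AimBow function toggles character rotation mode but is not called here.
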(event Input|EnhancedActionEvents|EnhancedInputActionIA_Combat
  (params (ActionValue :type Boolean) (ElapsedSeconds :type Float%20%28double-precision%29) (TriggeredSeconds :type Float%20%28double-precision%29) (InputAction :type Input%20Action%20Object%20Reference :default "/Game/Core/Input/Actions/IA_Combat.IA_Combat"))
  (bind _swordref (Variables|Default|GetSwordRef))
  (bind _sword (Variables|/Game/Blueprint/Object/BP_Sword.BP_Sword_C|GetSword _swordref))
  (:Started
    (if (and (Components|Activation|IsActive) (not (Variables|Default|GetbIsPerformAttack)))
      (Development|PrintString "AttackSword")
      (Development|SetHiddeninGame (Variables|/Game/Blueprint/Object/BP_Sword.BP_Sword_C|GetSword (Variables|Default|GetSwordRef)) false false)
      (Variables|Default|SetAttackIndex (Math|Integer|%(Integer) (+ (Variables|Default|GetAttackIndex) 1) (Utilities|Array|Length (Variables|Default|GetAttacks))))
      (Animation|Montage|PlayMontage (Variables|/Script/Engine.Character|GetMesh (Variables|Default|GetCharacter_0)) (Utilities|Array|Get(acopy) (Variables|Default|GetAttacks) (Variables|Default|GetAttackIndex)) 0.9
        (:then
          (Variables|Default|SetbIsPerformAttack true))
        (:OnCompleted
          (Variables|Default|SetbIsPerformAttack false)))
      (else
        (Utilities|IsValid _sword
          (:Is%20Valid
            (Development|SetHiddeninGame _sword true true)))))))

(event EventBeginPlay
  (Utilities|FlowControl|Delay 1.0)
  (bind _character (CallFunction|GetCharacter))
  (Variables|Default|SetCharacter_0 _character)
  (bind _returnvalue (Actor|GetActorOfClass "/Game/Blueprint/Object/BP_Sword.BP_Sword_C"))
  (Variables|Default|SetSwordRef _returnvalue)
  (bind _returnvalue_2 (Game|SpawnActorfromClass "/Game/Blueprint/Object/BP_Sword.BP_Sword_C" (Variables|Default|GetSpawn%20Transform) "Undefined" "MultiplyWithRoot" 0 0))
  (bind _output_get (Variables|Default|SetSwordRef _returnvalue_2))
  (Transformation|AttachComponentToComponent _output_get (Variables|/Script/Engine.Character|GetMesh (Variables|Default|GetCharacter_0)) "sword" "SnapToTarget" "SnapToTarget" "SnapToTarget" true)
  (Development|SetHiddeninGame (Variables|/Game/Blueprint/Object/BP_Sword.BP_Sword_C|GetSword (Variables|Default|GetSwordRef)) true false))

(fn StartAbility
  (|CallParentFunction)
  (CallFunction|LogBoolean "AttackSword StartAblity" (Components|Activation|IsActive) "(R=0.000000,G=1.000000,B=0.000000,A=1.000000)" "(R=1.000000,G=0.000000,B=0.000000,A=1.000000)"))

(fn StopAbility
  (|CallParentFunction)
  (CallFunction|LogBoolean "AttackSword StopAblity" (Components|Activation|IsActive) "(R=0.000000,G=1.000000,B=0.000000,A=1.000000)" "(R=1.000000,G=0.000000,B=0.000000,A=1.000000)"))

(fn AimBow
  (params (Toogle :type Boolean))
  (bind _character_0 (Variables|Default|GetCharacter_0))
  (bind _character_0_2 (Variables|Default|GetCharacter_0))
  (bind _charactermovement (Variables|/Script/Engine.Character|GetCharacterMovement _character_0))
  (bind _charactermovement_2 (Variables|/Script/Engine.Character|GetCharacterMovement _character_0_2))
  (if Toogle
    (Variables|/Script/Engine.CharacterMovementComponent|SetbOrientRotationToMovement _charactermovement false)
    (Variables|/Script/Engine.CharacterMovementComponent|SetbUseControllerDesiredRotation _charactermovement true)
    (Variables|/Script/Engine.CharacterMovementComponent|SetRotationRate _charactermovement "0.000000,3000.000000,0.000000")
    (else
      (Variables|/Script/Engine.CharacterMovementComponent|SetbOrientRotationToMovement _charactermovement_2 true)
      (Variables|/Script/Engine.CharacterMovementComponent|SetbUseControllerDesiredRotation _charactermovement_2 false)
      (Variables|/Script/Engine.CharacterMovementComponent|SetRotationRate _charactermovement_2 "0.000000,5000.000000,0.000000"))))

(fn GetCharacter
  (bind _character (|CallParentFunction))
  (return _character))
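; Player combat component that handles a melee combo and equips the owning Character with a sword.
; On BeginPlay it spawns BP_Epée and attaches it to the right-hand socket of the Character mesh.
; Each IA_Combat press plays the next montage from the Attacks array on that mesh.
; A retriggerable delay resets the combo counter after inactivity, and reaching the last attack resets it immediately.
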(event Custom|Reset%20Attack%20Combo
  (Variables|Default|SetAttackCombo 0))

(event Custom|Perform%20Attack
  (Math|Integer|IncrementInt (Variables|Default|GetAttackCombo)
    (:%20%20
      (Utilities|FlowControl|RetriggerableDelay 2.0)
      (Variables|Default|SetAttackCombo 0))))

(event Input|EnhancedActionEvents|EnhancedInputActionIA_Combat
  (params (ActionValue :type Boolean) (ElapsedSeconds :type Float%20%28double-precision%29) (TriggeredSeconds :type Float%20%28double-precision%29) (InputAction :type Input%20Action%20Object%20Reference :default "/Game/Core/Input/Actions/IA_Combat.IA_Combat"))
  (:Started
    (bind _animationmontage (CallFunction|PerformCombo))
    (Animation|Montage|PlayMontage (Variables|/Script/Engine.Character|GetMesh (stale EventBeginPlay _ascharacter)) _animationmontage 0.9)))

(event EventBeginPlay
  (bind _ascharacter (Utilities|Casting|CastToCharacter (Components|GetOwner)))
  (bind _returnvalue (Game|SpawnActorfromClass "/Game/Blueprint/Object/BP_Epée.BP_Epée_C" (Variables|Default|GetSpawn%20Transform) "Undefined" "MultiplyWithRoot" 0 0))
  (Transformation|AttachComponentToComponent _returnvalue (Variables|/Script/Engine.Character|GetMesh _ascharacter) "hand_rSocket" "SnapToTarget" "SnapToTarget" "KeepRelative" true))

(event EventTick
  (params (DeltaSeconds :type Float%20%28single-precision%29)))

(fn PerformCombo
  (bind _attacks (Variables|Default|GetAttacks))
  (if (>= (Variables|Default|GetAttackCombo) (- (Utilities|Array|Length (Variables|Default|GetAttacks)) 1))
    (CallFunction|ResetAttackCombo)
    (return (Utilities|Array|Get(acopy) _attacks (Utilities|Array|LastIndex _attacks)))
    (else
      (CallFunction|PerformAttack)
      (return (Utilities|Array|Get(acopy) (Variables|Default|GetAttacks) (- (Variables|Default|GetAttackCombo) 1))))))
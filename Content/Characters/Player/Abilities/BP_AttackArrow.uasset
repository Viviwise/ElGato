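; Player ability component for bow combat that spawns a bow on the character's mesh socket and handles aiming and shooting.
; Combat input, while active, switches rotation to controller yaw, shows a crosshair, attaches an arrow and zooms FOV through a tick that disables itself once settled.
; Attack input launches the arrow toward a camera trace target and plays a shoot-and-draw montage, with Redraw spawning the next arrow while aiming.
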(event Custom|Redraw
  (Variables|Default|GetArrow
    (:then)
    (:else
      (if (Variables|Default|GetIsanimating)
        (Default|DrawBow (Variables|Default|GetBowRef))
        (bind _returnvalue (Game|SpawnActorfromClass "/Game/Blueprint/BP_Bow.BP_Bow_C" (Math|Transform|MakeTransform "0, 0, 0" "0, 0, 0" "1.000000,1.000000,1.000000") "Undefined" "MultiplyWithRoot" 0 0))
        (bind _output_get (Variables|Default|SetArrow _returnvalue))
        (Transformation|AttachComponentToComponent _output_get (Variables|/Script/Engine.Character|GetMesh (Variables|Default|GetCharacter_0)) "arrow" "SnapToTarget" "SnapToTarget" "SnapToTarget" false)
        (Development|SetHiddeninGame (Variables|/Game/Blueprint/BP_BowWeapon.BP_BowWeapon_C|GetSkeletalMesh (Variables|Default|GetBowRef)) false false)
        (Collision|SetActorEnableCollision (Variables|Default|GetArrow) false)))))

(event Custom|StartZoom
  (Variables|Default|SetTargetFOV (Variables|Default|GetZoomFov))
  (Components|Tick|SetComponentTickEnabled true))

(event Custom|StopZoom
  (Variables|Default|SetTargetFOV (Variables|Default|GetDefaultFov))
  (Components|Tick|SetComponentTickEnabled true))

(event Input|EnhancedActionEvents|EnhancedInputActionIA_Combat
  (params (ActionValue :type Boolean) (ElapsedSeconds :type Float%20%28double-precision%29) (TriggeredSeconds :type Float%20%28double-precision%29) (InputAction :type Input%20Action%20Object%20Reference :default "/Game/Core/Input/Actions/IA_Combat.IA_Combat"))
  (:Started
    (if (Components|Activation|IsActive)
      (Variables|Default|SetMovementState "NewEnumerator2")
      (CallFunction|AimBow true)
      (CallFunction|StartZoom)
      (bind _returnvalue (Game|SpawnActorfromClass "/Game/Blueprint/BP_Bow.BP_Bow_C" (Math|Transform|MakeTransform "0, 0, 0" "0, 0, 0" "1.000000,1.000000,1.000000") "Undefined" "MultiplyWithRoot" 0 0))
      (bind _output_get (Variables|Default|SetArrow _returnvalue))
      (Transformation|AttachComponentToComponent _output_get (Variables|/Script/Engine.Character|GetMesh (Variables|Default|GetCharacter_0)) "arrow" "SnapToTarget" "SnapToTarget" "SnapToTarget" false)
      (Development|SetHiddeninGame (Variables|/Game/Blueprint/BP_BowWeapon.BP_BowWeapon_C|GetSkeletalMesh (Variables|Default|GetBowRef)) false false)
      (Collision|SetActorEnableCollision (Variables|Default|GetArrow) false)
      (else
        (Variables|Default|SetMovementState "NewEnumerator0")
        (Development|PrintString "Desactivate arow")
        (Development|SetHiddeninGame (Variables|/Game/Blueprint/BP_BowWeapon.BP_BowWeapon_C|GetSkeletalMesh (Variables|Default|GetBowRef)) true false)
        (Collision|SetActorEnableCollision (Variables|Default|GetBowRef) false))))
  (:Completed
    (CallFunction|AimBow false)
    (CallFunction|StopZoom)
    (bind _arrow (Variables|Default|GetArrow)
      (:then
        (Actor|DestroyActor _arrow))
      (:else))))

(event Input|EnhancedActionEvents|EnhancedInputActionIA_ChargeAttackWeapon
  (params (ActionValue :type Boolean) (ElapsedSeconds :type Float%20%28double-precision%29) (TriggeredSeconds :type Float%20%28double-precision%29) (InputAction :type Input%20Action%20Object%20Reference :default "/Game/Variant_Combat/Input/Actions/IA_ChargeAttackWeapon.IA_ChargeAttackWeapon"))
  (:Started
    (bind _arrow (Variables|Default|GetArrow)
      (:then
        (Transformation|DetachFromActor _arrow "KeepWorld" "KeepWorld" "KeepWorld")
        (Default|LauckArrow _arrow (CallFunction|CaculateArrowVelocity))
        (Collision|SetActorEnableCollision (Variables|Default|GetArrow) true)
        (Animation|Montage|PlayMontage (Variables|/Script/Engine.Character|GetMesh (Variables|Default|GetCharacter_0)) "/Game/Animation/AnimationsBow/AR_ShootAndDraw_Montage.AR_ShootAndDraw_Montage"
          (:then
            (Default|FiredBow (Variables|Default|GetBowRef))
            (Variables|Default|SetArrow 0)
            (Development|PrintString "Collision retrouvé "))))
      (:else))))

(event EventBeginPlay
  (Utilities|FlowControl|Sequence
    (:then_0
      (bind _character (CallFunction|GetCharacter))
      (Variables|Default|SetCharacter_0 _character)
      (Variables|Default|SetCamera (Variables|/Game/Characters/Player/BP_Character.BP_Character_C|GetCamera (Variables|Default|GetCharacter_0))))
    (:then_1
      (Variables|Default|SetCurrentFov 9e+01)
      (Variables|Default|SetTargetFOV 9e+01)
      (Components|Tick|SetComponentTickEnabled false))
    (:then_2
      (bind _returnvalue (Game|SpawnActorfromClass "/Game/Blueprint/BP_BowWeapon.BP_BowWeapon_C" (Math|Conversions|ToTransform(Vector) (Transformation|GetSocketLocation (Variables|/Script/Engine.Character|GetMesh (Variables|Default|GetCharacter_0)) "Bow")) "Undefined" "MultiplyWithRoot" 0 0))
      (bind _output_get (Variables|Default|SetBowRef _returnvalue))
      (Transformation|AttachComponentToComponent _output_get (Variables|/Script/Engine.Character|GetMesh (Variables|Default|GetCharacter_0)) "Bow" "SnapToTarget" "SnapToTarget" "SnapToTarget" false)
      (Development|PrintString "Desactivate arow")
      (Development|SetHiddeninGame (Variables|/Game/Blueprint/BP_BowWeapon.BP_BowWeapon_C|GetSkeletalMesh (Variables|Default|GetBowRef)) true true))
    (:then_3
      (bind _returnvalue_2 (UserInterface|CreateWidget "/Game/UI/Widgets/CursorBow.CursorBow_C"))
      (Variables|Default|SetCrosshair _returnvalue_2))))

(event EventTick
  (params (DeltaSeconds :type Float%20%28single-precision%29))
  (Development|PrintString (Utilities|String|Append "AttackArrow Tick : " (Utilities|String|ToString(Integer) (Math|Random|RandomInteger 1000))) true true "(R=0.000000,G=0.660000,B=1.000000,A=1.000000)" 2.0 "AttackArrowTick")
  (bind _output_get (Variables|Default|SetCurrentFov (Math|Interpolation|FInterpTo (Variables|Default|GetCurrentFov) (Variables|Default|GetTargetFOV) DeltaSeconds (Variables|Default|GetInterpSpeed))))
  (Camera|SetFieldOfView (Variables|/Game/Characters/Player/BP_Character.BP_Character_C|GetCamera (Variables|Default|GetCharacter_0)) _output_get)
  (if (< (Math|Float|Absolute(Float) (- (Variables|Default|GetCurrentFov) (Variables|Default|GetTargetFOV))) 0.1)
    (Components|Tick|SetComponentTickEnabled false)))

(fn GetCharacter
  (bind _character (|CallParentFunction))
  (return _character))

(fn StartDraw
  (Variables|Default|SetIsanimating true))

(fn EnterArrowMode)

(fn AimBow
  (params (ToggleAim :type Boolean))
  (bind _character_0 (Variables|Default|GetCharacter_0))
  (bind _character_0_2 (Variables|Default|GetCharacter_0))
  (bind _bowref (Variables|Default|GetBowRef))
  (bind _charactermovement (Variables|/Script/Engine.Character|GetCharacterMovement _character_0))
  (bind _charactermovement_2 (Variables|/Script/Engine.Character|GetCharacterMovement _character_0_2))
  (if ToggleAim
    (Variables|/Script/Engine.CharacterMovementComponent|SetbOrientRotationToMovement _charactermovement_2 false)
    (Variables|/Script/Engine.CharacterMovementComponent|SetbUseControllerDesiredRotation _charactermovement_2 true)
    (Variables|/Script/Engine.CharacterMovementComponent|SetRotationRate _charactermovement_2 "0.000000,3000.000000,0.000000")
    (Variables|Default|SetIsanimating true)
    (Default|DrawBow _bowref)
    (UserInterface|Viewport|AddtoViewport (Variables|Default|GetCrosshair) 0)
    (else
      (Variables|/Script/Engine.CharacterMovementComponent|SetbOrientRotationToMovement _charactermovement true)
      (Variables|/Script/Engine.CharacterMovementComponent|SetbUseControllerDesiredRotation _charactermovement false)
      (Variables|/Script/Engine.CharacterMovementComponent|SetRotationRate _charactermovement "0.000000,500.000000,0.000000")
      (Variables|Default|SetIsanimating false)
      (Default|FiredBow _bowref)
      (Widget|RemovefromParent (Variables|Default|GetCrosshair)))))

(fn CaculateArrowVelocity
  (bind _character_0 (Variables|Default|GetCharacter_0))
  (bind _camera (Variables|/Game/Characters/Player/BP_Character.BP_Character_C|GetCamera _character_0))
  (bind _returnvalue (Transformation|GetWorldLocation _camera))
  (bind (_outhit _returnvalue_2) (Collision|LineTraceByChannel _returnvalue (+ _returnvalue (* (Math|Vector|GetForwardVector _camera) 7e+03)) "TraceTypeQuery1" false 0 "ForDuration"))
  (bind _arrow (Variables|Default|GetArrow)
    (:then
      (return (Math|Vector|GetUnitDirection(Vector) (Transformation|GetActorLocation _arrow) (Math|Vector|SelectVector (.Location (Collision|BreakHitResult _outhit)) (.TraceEnd (Collision|BreakHitResult _outhit)) _returnvalue_2))))
    (:else)))
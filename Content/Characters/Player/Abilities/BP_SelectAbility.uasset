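; BP_SelectAbility switches the player's active ability between arrow attack, sword attack and normal components found on its owner.
; After a one-second delay on BeginPlay it fills the Weapons array and makes the first switch.
; Mouse wheel and debug-style keys pass index offsets to SwitchWeapon, which stops the current ability and starts the new one.
; NormalizeWeaponIndex is meant to wrap the index, but its modulo formula is marked unused.
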(event EventBeginPlay
  (bind _returnvalue (Components|GetOwner))
  (Utilities|FlowControl|Delay 1.0)
  (Utilities|Array|Add (Variables|Default|GetWeapons) (Actor|GetComponentbyClass _returnvalue "/Game/Characters/Player/Abilities/BP_AttackArrow.BP_AttackArrow_C"))
  (Utilities|Array|Add (Variables|Default|GetWeapons) (Actor|GetComponentbyClass _returnvalue "/Game/Characters/Player/Abilities/BP_AttackSword.BP_AttackSword_C"))
  (Utilities|Array|Add (Variables|Default|GetWeapons) (Actor|GetComponentbyClass _returnvalue "/Game/Characters/Player/Abilities/BP_Normal.BP_Normal_C"))
  (CallFunction|SwitchWeapon 1))

(event Input|MouseEvents|MouseWheelUp
  (params (Key :type Key%20Structure :default "None"))
  (:Pressed
    (CallFunction|SwitchWeapon 1)))

(event Input|MouseEvents|MouseWheelDown
  (params (Key :type Key%20Structure :default "None"))
  (:Pressed
    (CallFunction|SwitchWeapon -1)))

(event Input|KeyboardEvents|J
  (params (Key :type Key%20Structure :default "None"))
  (:Pressed
    (CallFunction|SwitchWeapon -1)))

(event Input|KeyboardEvents|K
  (params (Key :type Key%20Structure :default "None")))

(event Input|KeyboardEvents|L
  (params (Key :type Key%20Structure :default "None"))
  (:Pressed
    (CallFunction|SwitchWeapon 2)))

(event Input|KeyboardEvents|M
  (params (Key :type Key%20Structure :default "None"))
  (:Pressed
    (CallFunction|SwitchWeapon)))

(fn SwitchWeapon
  (params (AddIndex :type Integer))
  (bind _weapon (Utilities|GetWeapon (Variables|Default|GetCurrentIndex))
    (:True
      (Default|StopAbility _weapon))
    (:False
      _))
  (bind _output_get (Variables|Default|SetCurrentIndex (Utilities|NormalizeWeaponIndex (+ (Variables|Default|GetCurrentIndex) AddIndex))))
  (bind _weapon_2 (Utilities|GetWeapon _output_get)
    (:True
      (Default|StartAbility _weapon_2)
      (Development|PrintString (Utilities|String|Append "Weapon" (Utilities|GetDisplayName _weapon_2))))))
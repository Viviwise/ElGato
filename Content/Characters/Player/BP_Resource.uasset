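; Generic player resource Blueprint that tracks a clamped value, starts it at maximum and regenerates it over time.
; Consume, per-frame Drain and Restore route through SetValue, which fires OnChanged and prints a debug readout.
; A looping timer at the RegenDelay interval restores RegenRate times the seconds past NextRegenTime, which consumption pushes forward to delay regeneration.
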(event EventBeginPlay
  (CallFunction|SetValue (Variables|Default|GetMaxValue))
  (CallFunction|StartRegeneration))

(fn SetValue
  (params (NextValue :type Float%20%28double-precision%29))
  (bind _maxvalue (Variables|Default|GetMaxValue))
  (bind _returnvalue (Math|Float|Clamp(Float) NextValue 0.0 _maxvalue))
  (LocalVariables|SetOldValue (Variables|Default|GetCurrentValue))
  (Variables|Default|SetCurrentValue _returnvalue)
  (Default|CallOnChanged _returnvalue (LocalVariables|GetOldValue) (Variables|Default|GetMaxValue))
  (CallFunction|Debug)
  (return _returnvalue))

(fn Consume
  (params (Amount :type Float%20%28double-precision%29) (bConsumeToZero :type Boolean))
  (bind _currentvalue (Variables|Default|GetCurrentValue))
  (bind _returnvalue (- _currentvalue Amount))
  (bind _output_get (LocalVariables|SetbIsSuccess (> _returnvalue 0.0)))
  (if (or _output_get bConsumeToZero)
    (CallFunction|SetValue (Math|Float|Max(Float) _returnvalue 0.0))
    (Variables|Default|SetNextRegenTime (+ (Utilities|Time|GetTimeSeconds) (Variables|Default|GetRegenDelay))))
  (return (Variables|Default|GetCurrentValue) (LocalVariables|GetbIsSuccess)))

(fn Drain
  (params (DrainRate :type Float%20%28double-precision%29) (bDrainToZero :type Boolean))
  (bind (_value _bsuccess) (CallFunction|Consume (* DrainRate (Utilities|Time|GetWorldDeltaSeconds)) bDrainToZero))
  (return _value _bsuccess))

(fn Restore
  (params (Amount :type Float%20%28double-precision%29))
  (bind _value (CallFunction|SetValue (+ (Variables|Default|GetCurrentValue) Amount)))
  (return _value))

(fn RestoreFull
  (bind _value (CallFunction|SetValue (Variables|Default|GetMaxValue)))
  (return _value))

(fn GetValue
  (return (Variables|Default|GetCurrentValue)))

(fn GetPercent
  (return (/ (Variables|Default|GetCurrentValue) (Variables|Default|GetMaxValue))))

(fn GetIsFull
  (return (>= (Variables|Default|GetCurrentValue) (Variables|Default|GetMaxValue))))

(fn GetIsEmpty
  (return (<= (Variables|Default|GetCurrentValue) 0.0)))

(fn GetIsNotEmpty
  (return (> (Variables|Default|GetCurrentValue) 0.0)))

(fn ProcessRegeneration
  (bind _returnvalue (Utilities|Time|GetTimeSeconds))
  (CallFunction|Restore (* (Variables|Default|GetRegenRate) (Math|Float|Max(Float) (- _returnvalue (Variables|Default|GetNextRegenTime)) 0.0)))
  (Variables|Default|SetNextRegenTime _returnvalue)
  (CallFunction|Debug)
  (return))

(fn StartRegeneration
  (CallFunction|StopRegeneration)
  (if (and (> (Variables|Default|GetRegenDelay) 0.0) (> (Variables|Default|GetRegenRate) 0.0))
    (bind _returnvalue (Utilities|Time|SetTimerbyFunctionName 0 "ProcessRegeneration" (Variables|Default|GetRegenDelay) true true))
    (Variables|Default|SetRegenTimerHandle _returnvalue)
    (return)))

(fn StopRegeneration
  (Utilities|Time|ClearandInvalidateTimerbyHandle (Variables|Default|GetRegenTimerHandle))
  (return))

(fn Debug
  (bind _name (Variables|Default|GetName))
  (Development|PrintString (Utilities|String|Append _name " : " (Utilities|String|ToString(Integer) (Math|Float|Round (Variables|Default|GetCurrentValue))) " / " (Utilities|String|ToString(Integer) (Math|Float|Round (Variables|Default|GetMaxValue)))) true true "(R=1.000000,G=1.000000,B=0.997134,A=1.000000)" 5.0 (Utilities|String|StringToName _name)))
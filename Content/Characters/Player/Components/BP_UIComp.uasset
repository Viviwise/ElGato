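; Player UI component that creates the main HUD and keeps the stat bars in sync with the owning character.
; After a short BeginPlay delay, it adds WBP_main to the viewport and binds to the character's Stamina, HP, Mana and XP change events.
; Stamina and Mana ratios update HUD bars, while HP updates the character's own LifeBarWidget.
; The XP handler is bound but empty.
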(event Custom|OnChangedMana
  (params (NewValue :type Float%20%28double-precision%29) (OldValue :type Float%20%28double-precision%29) (MaxValue :type Float%20%28double-precision%29))
  (Default|SetPercentageMana (Variables|/Game/UI/Widgets/WBP_main.WBP_main_C|GetWBP_Mana (Variables|Default|GetUIStamina)) (/ NewValue MaxValue)))

(event Custom|OnChangedStamina
  (params (NewValue :type Float%20%28double-precision%29) (OldValue :type Float%20%28double-precision%29) (MaxValue :type Float%20%28double-precision%29))
  (Default|UpdatePercent (Variables|/Game/UI/Widgets/WBP_main.WBP_main_C|GetWBP_Stamina (Variables|Default|GetUIStamina)) (/ NewValue MaxValue)))

(event Custom|OnChangedHP
  (params (NewValue :type Float%20%28double-precision%29) (OldValue :type Float%20%28double-precision%29) (MaxValue :type Float%20%28double-precision%29))
  (Default|SetLifePercentage (Variables|/Game/Characters/Player/BP_Character.BP_Character_C|GetLife%20Bar%20Widget (Variables|Default|GetCharacter)) (/ NewValue MaxValue)))

(event Custom|OnChangedXP
  (params (NewValue :type Float%20%28double-precision%29) (OldValue :type Float%20%28double-precision%29) (MaxValue :type Float%20%28double-precision%29)))

(event EventBeginPlay
  (Utilities|FlowControl|Delay 0.2)
  (bind _character (CallFunction|GetCharacter))
  (Variables|Default|SetCharacter _character)
  (Utilities|FlowControl|Sequence
    (:then_0
      (bind _returnvalue (UserInterface|CreateWidget "/Game/UI/Widgets/WBP_main.WBP_main_C"))
      (bind _output_get (Variables|Default|SetUIStamina _returnvalue))
      (UserInterface|Viewport|AddtoViewport _output_get 0))
    (:then_1
      (EventDispatchers|BindEventtoOnChanged (Variables|/Game/Characters/Player/BP_Character.BP_Character_C|GetStamina (Variables|Default|GetCharacter)) (delegate Custom|OnChangedStamina)))
    (:then_2
      (EventDispatchers|BindEventtoOnChanged (Variables|/Game/Characters/Player/BP_Character.BP_Character_C|GetHP (Variables|Default|GetCharacter)) (delegate Custom|OnChangedHP)))
    (:then_3
      (EventDispatchers|BindEventtoOnChanged (Variables|/Game/Characters/Player/BP_Character.BP_Character_C|GetMana (Variables|Default|GetCharacter)) (delegate Custom|OnChangedMana)))
    (:then_4
      (EventDispatchers|BindEventtoOnChanged (Variables|/Game/Characters/Player/BP_Character.BP_Character_C|GetXP (Variables|Default|GetCharacter)) (delegate Custom|OnChangedXP)))))